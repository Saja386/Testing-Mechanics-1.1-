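; BP_PatrolRaot is an enemy AI patrol route that supplies spline points as world-space destinations.
; IncrementPatrolRaot steps PatrolIndex by Direction, setting Direction backward when the index equals the point count plus one and forward at zero, for back-and-forth traversal.
; The upper check lies beyond the last valid point index.
; GetSplinePointAsWorldPosition returns the world location of the spline point at the current index.
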(event `Increment Patrol Raot`
  (bind _output_get (set `self.Patrol Index` (+ (`self.Direction`) (`self.Patrol Index`))))
  (if (== _output_get (- (`SplineComponent.GetNumberOfSplinePoints` (`self.Spline`)) -1))
    (set `self.Direction` -1)
    (elif (== (`self.Patrol Index`) 0)
      (set `self.Direction` 1))))

(fn `Get Spline point as world position `
  (returns (NewParam :type "Vector Structure"))
  (return (`SplineComponent.GetLocationAtSplinePoint` (`self.Spline`) (`self.Patrol Index`) "World")))

(fn `UserConstructionScript`)